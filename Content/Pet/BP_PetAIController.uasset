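; BP_PetAIController is the pet's AI controller, linking its will and obedience to a StateTree that runs its AI.
; On BeginPlay it binds to action changes from UPetWill and order changes from UPetObedience.
; Either change sends a Pet.Reevaluate event to the StateTree, so reevaluation is event-driven.
; Action changes also print the new action on screen.
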(event `self.ReceiveBeginPlay`
  (add `UPetWillComponent.OnActionChanged` (`self.UPetWill`) (delegate `HandleActionChanged`))
  (add `UPetObedienceComponent.OnOrderChanged` (`self.UPetObedience`) (delegate `HandleOrderChanged`)))

(event `HandleOrderChanged`
  (`StateTreeComponent.SendStateTreeEvent` (`self.StateTreeAI`) (make `StateTreeEvent` (struct :`TagName` "Pet.Reevaluate"))))

(event `HandleActionChanged`
  (params (NewAction :type "EPetAction Enum" :default "Follow"))
  (`KismetSystemLibrary.PrintString` (`|GetEnumeratorNameAsString` NewAction))
  (`StateTreeComponent.SendStateTreeEvent` (`self.StateTreeAI`) (make `StateTreeEvent` (struct :`TagName` "Pet.Reevaluate"))))

(fn `UserConstructionScript`)